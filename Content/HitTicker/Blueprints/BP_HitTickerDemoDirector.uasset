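; Demo director for HitTicker that simulates combat by spawning floating combat text on every BP_HitTickerTarget in the level.
; BeginPlay caches targets, applies budget, merge, stats and draw-distance settings, optionally opens the control panel, and starts a looping CombatStep timer.
; With AutoCombat on, each step rolls per target at HitsPerSecond, then picks miss, block, heal, DoT, crit or damage through fresh rolls against cumulative thresholds, scattered above the target.
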(event EventBeginPlay
  (bind _returnvalue (Game|GetPlayerController 0))
  (bind _outactors (Actor|GetAllActorsOfClass "/HitTicker/HitTicker/Blueprints/BP_HitTickerTarget.BP_HitTickerTarget_C"))
  (Variables|Default|SetTargets _outactors)
  (Class|HitTickerStatics|SetBudget (Variables|HitTickerRuntime|GetDrawBudget))
  (Class|HitTickerStatics|SetMergeEnabled (Variables|HitTickerRuntime|GetbMergeEnabled))
  (Class|HitTickerStatics|SetShowStats (Variables|HitTickerRuntime|GetbShowStats))
  (Class|HitTickerSubsystem|SetMaxDrawDistance (Subsystems|GetHitTickerSubsystem) (Variables|HitTickerRuntime|GetMaxDrawDistance))
  (if (Variables|DemoSetup|GetbShowControlPanel)
    (bind _returnvalue_2 (UserInterface|CreateWidget "/HitTicker/HitTicker/UI/WBP_HitTickerDemoPanel.WBP_HitTickerDemoPanel_C" _returnvalue))
    (UserInterface|Viewport|AddtoViewport _returnvalue_2 0)
    (Input|SetInputModeGameandUI _returnvalue 0 "DoNotLock" false false)
    (Variables|/Script/Engine.PlayerController|SetbShowMouseCursor _returnvalue true))
  (Utilities|Time|SetTimerbyFunctionName self "CombatStep" 0.1 true))

(event Collision|EventActorBeginOverlap
  (params (OtherActor :type Actor%20Object%20Reference)))

(event EventTick
  (params (DeltaSeconds :type Float%20%28single-precision%29)))

(fn ConstructionScript)

(fn CombatStep
  (bind _returnvalue (Math|Random|RandomFloat))
  (bind _hitscatter (Variables|DemoCombat|GetHitScatter))
  (bind _mindamage (Variables|DemoCombat|GetMinDamage))
  (bind _maxdamage (Variables|DemoCombat|GetMaxDamage))
  (bind _misschance (Variables|DemoCombat|GetMissChance))
  (bind _blockchance (Variables|DemoCombat|GetBlockChance))
  (bind _healchance (Variables|DemoCombat|GetHealChance))
  (bind _dotchance (Variables|DemoCombat|GetDotChance))
  (bind _returnvalue_2 (+ _misschance _blockchance))
  (bind _returnvalue_3 (+ _returnvalue_2 _healchance))
  (bind _returnvalue_4 (+ _returnvalue_3 _dotchance))
  (if (not (not (Variables|DemoCombat|GetbAutoCombat)))
    (for _array_element (Variables|Default|GetTargets)
      (if (< (Math|Random|RandomFloat) (* (Variables|DemoCombat|GetHitsPerSecond) (Math|Float|MakeLiteralFloat 0.1)))
        (if (< _returnvalue _misschance)
          (Class|HitTickerStatics|AddCombatText (Math|Random|RandomPointinBoundingBox (+ (Transformation|GetActorLocation _array_element) (Math|Vector|MakeVector 0.0 0.0 (Variables|DemoCombat|GetHitHeight))) (Math|Vector|MakeVector _hitscatter _hitscatter (* _hitscatter (Math|Float|MakeLiteralFloat 0.6)))) "MISS" "Miss" _array_element)
          (elif (< _returnvalue _returnvalue_2)
            (Class|HitTickerStatics|AddCombatText (Math|Random|RandomPointinBoundingBox (+ (Transformation|GetActorLocation _array_element) (Math|Vector|MakeVector 0.0 0.0 (Variables|DemoCombat|GetHitHeight))) (Math|Vector|MakeVector _hitscatter _hitscatter (* _hitscatter (Math|Float|MakeLiteralFloat 0.6)))) "BLOCK" "Block" _array_element)
            (elif (< _returnvalue _returnvalue_3)
              (Class|HitTickerStatics|AddHealNumber (Math|Random|RandomPointinBoundingBox (+ (Transformation|GetActorLocation _array_element) (Math|Vector|MakeVector 0.0 0.0 (Variables|DemoCombat|GetHitHeight))) (Math|Vector|MakeVector _hitscatter _hitscatter (* _hitscatter (Math|Float|MakeLiteralFloat 0.6)))) (Math|Random|RandomFloatinRange (* _mindamage (Math|Float|MakeLiteralFloat 0.6)) _maxdamage) _array_element)
              (elif (< _returnvalue _returnvalue_4)
                (Class|HitTickerStatics|AddDamageOverTimeNumber (Math|Random|RandomPointinBoundingBox (+ (Transformation|GetActorLocation _array_element) (Math|Vector|MakeVector 0.0 0.0 (Variables|DemoCombat|GetHitHeight))) (Math|Vector|MakeVector _hitscatter _hitscatter (* _hitscatter (Math|Float|MakeLiteralFloat 0.6)))) (Math|Random|RandomFloatinRange 6.0 28.0) _array_element)
                (elif (< _returnvalue (+ _returnvalue_4 (Variables|DemoCombat|GetCritChance)))
                  (Class|HitTickerStatics|AddCritNumber (Math|Random|RandomPointinBoundingBox (+ (Transformation|GetActorLocation _array_element) (Math|Vector|MakeVector 0.0 0.0 (Variables|DemoCombat|GetHitHeight))) (Math|Vector|MakeVector _hitscatter _hitscatter (* _hitscatter (Math|Float|MakeLiteralFloat 0.6)))) (* (Math|Random|RandomFloatinRange _mindamage _maxdamage) (Variables|DemoCombat|GetCritMultiplier)) _array_element)
                  (else
                    (Class|HitTickerStatics|AddDamageNumber (Math|Random|RandomPointinBoundingBox (+ (Transformation|GetActorLocation _array_element) (Math|Vector|MakeVector 0.0 0.0 (Variables|DemoCombat|GetHitHeight))) (Math|Vector|MakeVector _hitscatter _hitscatter (* _hitscatter (Math|Float|MakeLiteralFloat 0.6)))) (Math|Random|RandomFloatinRange _mindamage _maxdamage) _array_element)))))))))))