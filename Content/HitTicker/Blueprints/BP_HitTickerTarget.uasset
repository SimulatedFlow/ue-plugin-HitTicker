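; BP_HitTickerTarget is a target actor that drifts around the spot where it was placed.
; BeginPlay stores the home location, and Tick teleport-free sets an offset from it each frame using three Perlin noise samples of game time.
; Different speed factors and seed offsets per axis decorrelate the motion, scaled by BobSpeed, OrbitRadius horizontally and BobHeight vertically, with PhaseOffset shifting the pattern.
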(event EventBeginPlay
  (Variables|Default|SetHomeLocation (Transformation|GetActorLocation)))

(event Collision|EventActorBeginOverlap
  (params (OtherActor :type Actor%20Object%20Reference)))

(event EventTick
  (params (DeltaSeconds :type Float%20%28single-precision%29))
  (bind _returnvalue (Utilities|Time|GetGameTimeinSeconds))
  (bind _phaseoffset (Variables|Default|GetPhaseOffset))
  (bind _bobspeed (Variables|Default|GetBobSpeed))
  (bind _orbitradius (Variables|Default|GetOrbitRadius))
  (Transformation|SetActorLocation (+ (Variables|Default|GetHomeLocation) (Math|Vector|MakeVector (* (Class|KismetMathLibrary|PerlinNoise1D (+ (* _returnvalue (* _bobspeed (Math|Float|MakeLiteralFloat 0.35))) _phaseoffset)) _orbitradius) (* (Class|KismetMathLibrary|PerlinNoise1D (+ (* _returnvalue (* _bobspeed (Math|Float|MakeLiteralFloat 0.3))) (+ _phaseoffset (Math|Float|MakeLiteralFloat 41.3)))) _orbitradius) (* (Class|KismetMathLibrary|PerlinNoise1D (+ (* _returnvalue (* _bobspeed (Math|Float|MakeLiteralFloat 0.55))) (+ _phaseoffset (Math|Float|MakeLiteralFloat 13.7)))) (Variables|Default|GetBobHeight)))) false false))

(fn ConstructionScript)